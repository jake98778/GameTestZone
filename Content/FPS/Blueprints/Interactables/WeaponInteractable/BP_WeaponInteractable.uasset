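; A weapon pickup actor that shows a physics-simulated mesh for the weapon class in WeaponToSpawn.
; The RepNotify on WeaponToSpawn calls ShowMesh and applies a random rotation.
; ShowMesh uses the same rifle mesh for every named weapon, distinguishing the sniper, machinegun, rifle and shotgun classes by a material swap.
; Interact only casts the instigator to BP_BaseCharacter, and BeginHover returns false, so pickup logic is absent here.
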(event `/Game/FPS/Blueprints/Interfaces/iInteractive.Interact`
  (params (Instigator :type "Actor Object Reference"))
  ;[1 1 1] Interact
  (cast `/Game/FPS/Blueprints/CharacterAndClasses/BP_BaseCharacter` Instigator))

(event `ShowMesh`
  (bind _staticmesh (`self.StaticMesh`))
  (bind _weapontospawn (`self.WeaponToSpawn`))
  ;[1 1 1] Begin Play
  (`SceneComponent.SetVisibility` (`self.StaticMesh`) true false)
  (`PrimitiveComponent.SetSimulatePhysics` (`self.StaticMesh`) true)
  (switch `/Game/FPS/Blueprints/Weapons/EWeaponNames` (`.WeaponName` (defaults `Object` (`self.WeaponToSpawn`)))
    (:`NewEnumerator0`
      (set `self.WeaponMesh` "/Game/FPS/Assets/Weapons/SM_Rifle.SM_Rifle"))
    (:`NewEnumerator1`
      (set `self.WeaponMesh` "/Game/FPS/Assets/Weapons/SM_Rifle.SM_Rifle"))
    (:`NewEnumerator2`
      (set `self.WeaponMesh` "/Game/FPS/Assets/Weapons/SM_Rifle.SM_Rifle"))
    (:`NewEnumerator3`
      (set `self.WeaponMesh` "/Game/FPS/Assets/Weapons/SM_Rifle.SM_Rifle"))
    (:`NewEnumerator4`
      (set `self.WeaponMesh` "/Game/FPS/Assets/Weapons/SM_Rifle.SM_Rifle")))
  (`StaticMeshComponent.SetStaticMesh` (`self.StaticMesh`) (`self.WeaponMesh`))
  (if (== _weapontospawn "/Game/FPS/Blueprints/Weapons/BP_SniperRifle_Weapon.BP_SniperRifle_Weapon_C")
    (`PrimitiveComponent.SetMaterial` _staticmesh 3 "/Game/FPS/Textures/Materials/M_Base_Inst1.M_Base_Inst1")
    (elif (== _weapontospawn "/Game/FPS/Blueprints/Weapons/BP_Machinegun_Weapon.BP_Machinegun_Weapon_C")
      (`PrimitiveComponent.SetMaterial` _staticmesh 3 "/Game/FPS/Textures/Materials/M_Base_Inst2.M_Base_Inst2")
      (elif (== _weapontospawn "/Game/FPS/Blueprints/Weapons/BP_Rifle_Weapon.BP_Rifle_Weapon_C")
        (`PrimitiveComponent.SetMaterial` _staticmesh 3 "/Game/FPS/Textures/Materials/FlagMaterial_Inst3.FlagMaterial_Inst3")
        (elif (== _weapontospawn "/Game/FPS/Blueprints/Weapons/BP_Shotgun_Weapon.BP_Shotgun_Weapon_C")
          (`PrimitiveComponent.SetMaterial` _staticmesh 3 "/Game/FPS/Textures/Materials/FlagMaterial_Inst.FlagMaterial_Inst"))))))

(fn `BeginHover`
  (params (Instigator :type "Actor Object Reference"))
  (returns (bFailure :type Boolean))
  (return false))

(fn `OnRep_WeaponToSpawn`
  (`self.ShowMesh`)
  (`self.K2_SetActorRotation` (`KismetMathLibrary.RandomRotator` false)))

(fn `UserConstructionScript`
  (`parent.UserConstructionScript`))