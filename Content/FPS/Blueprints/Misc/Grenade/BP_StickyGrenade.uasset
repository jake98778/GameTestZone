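; BP_StickyGrenade is a grenade that sticks to what it hits and beeps until it explodes.
; On a sphere hit, the server multicasts the audio start and attaches the grenade to the valid hit actor at the hit bone, keeping its world transform.
; A looping timer replays a high-pitched shutter sound until exploded.
; On explosion it destroys its light, health and projectile movement components and hides the mesh.
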(event `self.Sphere.OnComponentHit`
  (params (HitComponent :type "PrimitiveComponent Object Reference") (OtherActor :type "Actor Object Reference") (OtherComp :type "PrimitiveComponent Object Reference") (NormalImpulse :type "Vector Structure") (Hit :type "HitResult Structure (by ref)"))
  ;[1 1 1] On hit
  (`/Engine/EditorBlueprintResources/ActorMacros.Switch Has Authority`
    (:`Authority`
      (`self.Multicast_ActivateAudio`)
      (`/Engine/EditorBlueprintResources/StandardMacros.IsValid` OtherActor
        (:`Is Valid`
          (`self.AttachToActor` OtherActor Hit_HitBoneName))))))

(event `Multicast_ActivateAudio`
  ;[1 1 1] Multicast Play Audio
  (`self.PlayAudio`)
  (`KismetSystemLibrary.K2_SetTimerDelegate` (delegate `PlayAudio`) 0.7 true))

(event `AttachToActor`
  (params (Actor :type "Actor Object Reference") (BoneName :type Name))
  ;[1 1 1] Attach grenade
  (`self.K2_AttachToActor` Actor BoneName "KeepWorld" "KeepWorld" "KeepWorld"))

(event `self.OnExploded`
  ;[1 1 1] Attach grenade
  (`ActorComponent.K2_DestroyComponent` (`self.PointLight`))
  (`ActorComponent.K2_DestroyComponent` (`self.HealthComponent`))
  (`ActorComponent.K2_DestroyComponent` (`self.ProjectileMovement`))
  (`SceneComponent.SetVisibility` (`self.Mesh`) false false))

(event `PlayAudio`
  ;[1 1 1] Multicast Play Audio
  (if (not (`self.bExploded`))
    (`GameplayStatics.PlaySoundAtLocation` "/Engine/VREditor/Sounds/UI/Camera_Shutter.Camera_Shutter" (`self.K2_GetActorLocation`) (struct) 0.2 2.0 0.0 "/Game/FPS/MusicSound/Sounds/WeaponAttenuation.WeaponAttenuation" null null)))

(fn `UserConstructionScript`
  (`parent.UserConstructionScript`))