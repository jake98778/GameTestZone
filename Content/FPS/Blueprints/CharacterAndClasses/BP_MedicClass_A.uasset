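; Medic character class for the FPS, whose class skill spawns a team-assigned medic bot.
; UseClassSkill checks availability, then calls a server event that spawns BP_MedicBot high above the pawn with its team and owner set.
; The bot's lifespan equals the ability cooldown.
; A timer re-enables the skill, and player controller 0's gameplay widget is notified on use and reset.
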(event `self.ReceiveBeginPlay`
  (`parent.ReceiveBeginPlay`))

(event `self.ReceiveTick`
  (params (DeltaSeconds :type "Float (single-precision)"))
  (`parent.ReceiveTick` DeltaSeconds))

(event `ResetSkill`
  ;[1 1 1] Reset Skill
  (set `self.bCanUseSkill` true)
  (`/Game/FPS/WidgetBP/WB_Gameplay.SkillReset` (`/Game/FPS/Blueprints/PlayerController/BasePlayerController.GameplayWBRef` (cast `/Game/FPS/Blueprints/PlayerController/BasePlayerController` (`GameplayStatics.GetPlayerController` 0) :!pure true))))

(event `self.UseClassSkill`
  (bind _asbase_player_controller (cast `/Game/FPS/Blueprints/PlayerController/BasePlayerController` (`GameplayStatics.GetPlayerController` 0) :!pure true))
  ;[1 1 1] Medic Skill
  (if (`self.bCanUseSkill`)
    (set `self.bCanUseSkill` false)
    (`self.Server_SpawnMedicBot` self (`/Game/FPS/Blueprints/PlayerController/BasePlayerController.bTeam` _asbase_player_controller))
    (`GameplayStatics.PlaySound2D` "/Engine/VREditor/Sounds/UI/Invalid_Action.Invalid_Action" 1.0 1.0 0.0 null null)
    (bind _returnvalue (`KismetSystemLibrary.K2_SetTimerDelegate` (delegate `ResetSkill`) (`self.AbilityCoolDown`)))
    (`/Game/FPS/WidgetBP/WB_Gameplay.OnSkillUsed` (`/Game/FPS/Blueprints/PlayerController/BasePlayerController.GameplayWBRef` _asbase_player_controller) _returnvalue)))

(event `Server_SpawnMedicBot`
  (params (Pawn :type "/Game/FPS/Blueprints/CharacterAndClasses/BP_BaseCharacter Object Reference") (bTeam :type Boolean))
  (bind (_returnvalue_x _returnvalue_y _returnvalue_z) (`KismetMathLibrary.BreakVector` (`self.K2_GetActorLocation` self)))
  ;[1 1 1] Spawn Medic Bot
  (bind _returnvalue (`|SpawnActorFromClass` "/Game/FPS/Blueprints/AI_Pawns/MedicBot/BP_MedicBot.BP_MedicBot_C" (`KismetMathLibrary.MakeTransform` (`KismetMathLibrary.MakeVector` _returnvalue_x _returnvalue_y (+ _returnvalue_z 1000.0)) (`self.K2_GetActorRotation` self)) "Undefined" "OverrideRootScale" Pawn (`self.AbilityCoolDown`) Pawn))
  (set `/Game/FPS/Blueprints/AI_Pawns/MedicBot/BP_MedicBot.bBotTeam` bTeam _returnvalue)
  (set `/Game/FPS/Blueprints/AI_Pawns/MedicBot/BP_MedicBot.OwnerPawn` self _returnvalue))

(fn `UserConstructionScript`
  (`parent.UserConstructionScript`))